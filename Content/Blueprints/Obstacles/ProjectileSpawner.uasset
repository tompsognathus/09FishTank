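; ProjectileSpawner is an obstacle Blueprint that repeatedly spawns projectiles at random points along a line.
; Tick counts down a timer, spawns an actor of ProjectileClass at zero, then rolls a new short random delay.
; Spawn points keep the X and Z of Arrow and interpolate Y randomly toward Arrow1.
; StartSpawning sets IsSpawning, but Tick never checks that flag.
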(event `self.ReceiveTick`
  (params (DeltaSeconds :type "Float (single-precision)"))
  (bind _output_get (set `self.TimeUntilNextSpawn` (- (`self.TimeUntilNextSpawn`) DeltaSeconds)))
  (if (<= _output_get 0.0)
    (bind _randomspawnworldlocation (`self.GenerateRandomSpawnLocation`))
    (`self.SpawnProjectile` _randomspawnworldlocation)
    (bind _timeuntilnextspawn (`self.GenerateTimeUntilNextSpawn`))
    (set `self.TimeUntilNextSpawn` _timeuntilnextspawn)))

(fn `GenerateRandomSpawnLocation`
  (returns (RandomSpawnWorldLocation :type "Vector Structure"))
  (bind (_returnvalue_x _returnvalue_y _returnvalue_z) (`KismetMathLibrary.BreakVector` (`SceneComponent.K2_GetComponentLocation` (`self.Arrow`))))
  (bind (_returnvalue_x_2 _returnvalue_y_2) (`KismetMathLibrary.BreakVector` (`SceneComponent.K2_GetComponentLocation` (`self.Arrow1`))))
  (bind _output_get (set `self.SpawnLocation` (`KismetMathLibrary.MakeVector` _returnvalue_x (+ _returnvalue_y (* (- _returnvalue_y_2 _returnvalue_y) (`KismetMathLibrary.RandomFloat`))) _returnvalue_z)))
  (return _output_get))

(fn `GenerateTimeUntilNextSpawn`
  (returns (TimeUntilNextSpawn :type "Float (double-precision)"))
  (return (+ (* (`KismetMathLibrary.RandomFloat`) 1.0) 0.2)))

(fn `SpawnProjectile`
  (params (SpawnLocation :type "Vector Structure"))
  (`|SpawnActorFromClass` (`self.ProjectileClass`) (`KismetMathLibrary.MakeTransform` SpawnLocation) "Undefined" "MultiplyWithRoot" null null))

(fn `StartSpawning`
  (set `self.IsSpawning` true))

(fn `UserConstructionScript`)