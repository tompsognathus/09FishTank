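; BP_Spike is a single-use spike obstacle that damages the player's fish on contact.
; When an actor tagged Player overlaps its Cone, it casts the player character to BP_FishParent, applies damage and plays a hit sound.
; It then teleports itself to the world origin, briefly shows the damage UI through UIManager, and destroys itself after the short delay.
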(event `self.Cone.OnComponentBeginOverlap`
  (params (OverlappedComponent :type "PrimitiveComponent Object Reference") (OtherActor :type "Actor Object Reference") (OtherComp :type "PrimitiveComponent Object Reference") (OtherBodyIndex :type Integer) (bFromSweep :type Boolean) (SweepResult :type "HitResult Structure (by ref)"))
  (if (`self.ActorHasTag` OtherActor "Player")
    (bind _asbp_fish_parent (cast `/Game/Blueprints/Fish/BP_FishParent` (`GameplayStatics.GetPlayerCharacter` 0)))
    (`/Game/Blueprints/Fish/BP_FishParent.TakeDamage` _asbp_fish_parent 10)
    (`GameplayStatics.PlaySound2D` "/Game/Audio/SFX/hit.hit" 1.0 1.0 0.0 null null)
    (`self.K2_SetActorLocation` (0.0 0.0 0.0))
    (bind _returnvalue (`GameplayStatics.GetActorOfClass` "/Script/HyperCasual.UIManager"))
    (`UIManager.OpenDamageUI` _returnvalue)
    (`KismetSystemLibrary.Delay` 0.2)
    (`UIManager.CloseDamageUI` _returnvalue)
    (`self.K2_DestroyActor`)))

(fn `UserConstructionScript`)